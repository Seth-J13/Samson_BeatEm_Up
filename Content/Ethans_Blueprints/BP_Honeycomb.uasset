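; BP_Honeycomb is a healing pickup that restores the player's health on touch and then removes itself.
; On BeginPlay it caches the player character as a BP_CombatCharacter.
; When that character overlaps the Box component, a DoOnce gate lets a single ApplyHealing interface message through before the actor is destroyed.
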(event OnComponentBeginOverlap(Box)
  (params (OverlappedComponent :type Primitive%20Component%20Object%20Reference) (OtherActor :type Actor%20Object%20Reference) (OtherComp :type Primitive%20Component%20Object%20Reference) (OtherBodyIndex :type Integer) (bFromSweep :type Boolean) (SweepResult :type Hit%20Result%20Structure%20%28by%20ref%29))
  (if (== OtherActor (Variables|Default|GetAs%20BP%20Combat%20Character))
    (Utilities|FlowControl|DoOnce false
      (:Completed
        (Class|BPIDamageable|ApplyHealing(Message) (Variables|Default|GetAs%20BP%20Combat%20Character) 1e+02)
        (Actor|DestroyActor)))))

(event EventBeginPlay
  (bind _asbp_combat_character (Utilities|Casting|CastToBP_CombatCharacter (Game|GetPlayerCharacter 0)))
  (Variables|Default|SetAs%20BP%20Combat%20Character _asbp_combat_character))

(event Collision|EventActorBeginOverlap
  (params (OtherActor :type Actor%20Object%20Reference)))

(event EventTick
  (params (DeltaSeconds :type Float%20%28single-precision%29)))

(fn ConstructionScript)